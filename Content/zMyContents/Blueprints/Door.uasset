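; Door Blueprint that raises and lowers its Wall component in response to Activate and Deactivate events.
; Activate plays a sound and runs a timeline that offsets the wall's Z from its starting location; Deactivate reverses it.
; With MultiSwitch on, Activate opens the door only when its counter reaches two, resetting above that.
; Deactivate decrements that counter only when MultiSwitch is off.
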(event `self.ReceiveBeginPlay`
  (set `self.InitDoorLocation` (`SceneComponent.K2_GetComponentLocation` (`self.Wall`))))

(event `/Game/zMyContents/Blueprints/SwitchInterface.Activate`
  (bind _switchnumber (`self.SwitchNumber`))
  (if (`self.MultiSwitch`)
    (`/Engine/EditorBlueprintResources/StandardMacros.IncrementInt` _switchnumber
      (:`  `
        (`KismetSystemLibrary.PrintString` (`KismetStringLibrary.Conv_IntToString` _switchnumber))
        (if (> _switchnumber 2)
          (set `self.SwitchNumber` 0))
        (if (== _switchnumber 2)
          (`GameplayStatics.PlaySound2D` "/Game/zMyContents/Audio/OpenGateSound.OpenGateSound" 1.0 1.0 0.0 null null :!label _label)
          (bind (_direction _doorelevation) (`Timeline|DoorTimeline` :!label _label_2)
            (:`Update`
              (`SceneComponent.K2_SetWorldLocation` (`self.Wall`) (`KismetMathLibrary.MakeVector` (.x (`self.InitDoorLocation`)) (.y (`self.InitDoorLocation`)) (+ (.z (`self.InitDoorLocation`)) _doorelevation)) false false))))))
    (else
      (goto _label))))

(event `/Game/zMyContents/Blueprints/SwitchInterface.Deactivate`
  (if (`self.MultiSwitch`)
    (goto _label_2 :!via `Reverse`)
    (else
      (`/Engine/EditorBlueprintResources/StandardMacros.DecrementInt` (`self.SwitchNumber`)
        (:`  `
          (goto _label_2 :!via `Reverse`))))))

(fn `UserConstructionScript`)