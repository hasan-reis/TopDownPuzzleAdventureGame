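; Player character Blueprint with Space to jump, navigation-based movement to a hit location, and a toggleable target icon.
; MoveToHitResult prints the distance to the given hit and sends the player controller there with SimpleMoveToLocation; its zero-distance threshold always passes.
; EnableTargetIcon and DisableTargetIcon show or hide the widget component and play or stop its looping TargetIconWidget_BP animation.
; The icon starts hidden on BeginPlay.
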(event `InputAction|Space`
  (params (Key :type "Key Structure"))
  (:`Pressed`
    (`self.Jump`)))

(event `self.ReceiveBeginPlay`
  (`self.DisableTargetIcon`))

(fn `DisableTargetIcon`
  (bind _widget (`self.Widget`))
  (bind _returnvalue (`WidgetComponent.GetUserWidgetObject` _widget))
  (bind _astarget_icon_widget_bp (cast `/Game/zMyContents/Blueprints/TargetIconWidget_BP` _returnvalue))
  (`UserWidget.StopAnimation` _returnvalue (`/Game/zMyContents/Blueprints/TargetIconWidget_BP.TargetIconAnim` _astarget_icon_widget_bp))
  (`SceneComponent.SetVisibility` _widget false false))

(fn `EnableTargetIcon`
  (bind _widget (`self.Widget`))
  (bind _returnvalue (`WidgetComponent.GetUserWidgetObject` _widget))
  (bind _astarget_icon_widget_bp (cast `/Game/zMyContents/Blueprints/TargetIconWidget_BP` _returnvalue))
  (`UserWidget.PlayAnimation` _returnvalue (`/Game/zMyContents/Blueprints/TargetIconWidget_BP.TargetIconAnim` _astarget_icon_widget_bp) 0.0 0 "Forward" 1.0 false)
  (`SceneComponent.SetVisibility` _widget true false))

(fn `Move to Hit Result`
  (params (HitResult :type "HitResult Structure"))
  (bind (_bblockinghit _binitialoverlap _time _distance _location) (`GameplayStatics.BreakHitResult` HitResult))
  (bind _returnvalue (`KismetMathLibrary.VSize` (- (`self.K2_GetActorLocation` (`GameplayStatics.GetPlayerPawn` 0)) _location)))
  (`KismetSystemLibrary.PrintString` (`KismetStringLibrary.Conv_DoubleToString` _returnvalue))
  (if (<= 0.0 _returnvalue)
    (`AIBlueprintHelperLibrary.SimpleMoveToLocation` (`GameplayStatics.GetPlayerController` 0) _location)))

(fn `UserConstructionScript`)