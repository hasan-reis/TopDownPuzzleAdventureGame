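; FloorSwitch is a pressure plate that the player triggers by stepping into its box trigger.
; Begin overlap sends ActivateMessage to each AffectedObjects entry implementing SwitchInterface, and end overlap sends DeactivateMessage.
; A timeline offsets the switch mesh vertically from its BeginPlay location, playing on entry and reversing on exit.
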(event `self.ReceiveBeginPlay`
  (set `self.InitSwitchLocation` (`SceneComponent.K2_GetComponentLocation` (`self.SwitchMesh`))))

(event `self.Box.OnComponentBeginOverlap`
  (params (OverlappedComponent :type "PrimitiveComponent Object Reference") (OtherActor :type "Actor Object Reference") (OtherComp :type "PrimitiveComponent Object Reference") (OtherBodyIndex :type Integer) (bFromSweep :type Boolean) (SweepResult :type "HitResult Structure (by ref)"))
  (cast `/Game/zMyContents/Blueprints/Player_BP` OtherActor)
  (for _array_element (`self.AffectedObjects`)
    (if (`KismetSystemLibrary.DoesImplementInterface` _array_element "/Game/zMyContents/Blueprints/SwitchInterface.SwitchInterface_C")
      (message `/Game/zMyContents/Blueprints/SwitchInterface.Activate` _array_element)))
  (bind (_direction _switchtrack) (`Timeline|Switch Timeline` :!label _label)
    (:`Update`
      (`SceneComponent.K2_SetWorldLocation` (`self.SwitchMesh`) (`KismetMathLibrary.MakeVector` (.x (`self.InitSwitchLocation`)) (.y (`self.InitSwitchLocation`)) (+ _switchtrack (.z (`self.InitSwitchLocation`)))) false false))))

(event `self.Box.OnComponentEndOverlap`
  (params (OverlappedComponent :type "PrimitiveComponent Object Reference") (OtherActor :type "Actor Object Reference") (OtherComp :type "PrimitiveComponent Object Reference") (OtherBodyIndex :type Integer))
  (cast `/Game/zMyContents/Blueprints/Player_BP` OtherActor)
  (for _array_element (`self.AffectedObjects`)
    (if (`KismetSystemLibrary.DoesImplementInterface` _array_element "/Game/zMyContents/Blueprints/SwitchInterface.SwitchInterface_C")
      (message `/Game/zMyContents/Blueprints/SwitchInterface.Deactivate` _array_element)))
  (goto _label :!via `Reverse`))

(fn `UserConstructionScript`)