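; Camera volume actor that blends the player's view to its own camera when Player_BP enters its box.
; The overlap stores the character and registers the volume on both player and controller.
; With UseSpline on, Tick moves the camera to the spline point closest to the character via VInterpTo, rotating it toward the volume's origin rather than the player.
; The direct look-at-player function is never run.
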(event `self.ReceiveTick`
  (params (DeltaSeconds :type "Float (single-precision)"))
  (set `self.Delta Seconds` DeltaSeconds)
  (if (`self.UseSpline`)
    (`self.CamRotateToPlayerWithSpline`)))

(event `self.ReceiveBeginPlay`
  (set `self.Controller` (`GameplayStatics.GetPlayerController` 0))
  (set `self.TurnUseSplineBackOn` (`self.UseSpline`))
  (set `self.InitialCameraTransform` (`SceneComponent.K2_GetComponentToWorld` (`self.Camera`))))

(event `self.Box.OnComponentBeginOverlap`
  (params (OverlappedComponent :type "PrimitiveComponent Object Reference") (OtherActor :type "Actor Object Reference") (OtherComp :type "PrimitiveComponent Object Reference") (OtherBodyIndex :type Integer) (bFromSweep :type Boolean) (SweepResult :type "HitResult Structure (by ref)"))
  (bind _controller (`self.Controller`))
  (bind _asplayer_bp (cast `/Game/zMyContents/Blueprints/Player_BP` OtherActor))
  (bind _output_get (set `self.Character` _asplayer_bp))
  (set `/Game/zMyContents/Blueprints/Player_BP.CurrentCameraVolume` self _output_get)
  (`/Engine/EditorBlueprintResources/StandardMacros.IsValid` _controller
    (:`Is Valid`
      (bind _asplayer_controller_bp (cast `/Game/zMyContents/Blueprints/PlayerController_BP` _controller))
      (set `/Game/zMyContents/Blueprints/PlayerController_BP.ControllerCurrentCameraVolume` self _asplayer_controller_bp)
      (`PlayerController.SetViewTargetWithBlend` (`self.Controller`) self 2.0 "VTBlend_Linear" 5.0 false))))

(fn `CamRotateToPlayer`
  (`/Engine/EditorBlueprintResources/StandardMacros.IsValid` (`self.Character`)
    (:`Is Valid`
      (`SceneComponent.K2_SetWorldRotation` (`self.Camera`) (`KismetMathLibrary.FindLookAtRotation` (`SceneComponent.K2_GetComponentLocation` (`self.Camera`)) (`self.K2_GetActorLocation` (`self.Character`))) false false))))

(fn `CamRotateToPlayerWithSpline`
  (bind _camera (`self.Camera`))
  (`/Engine/EditorBlueprintResources/StandardMacros.IsValid` (`self.Character`)
    (:`Is Valid`
      (`SceneComponent.K2_SetWorldLocationAndRotation` (`self.Camera`) (`KismetMathLibrary.VInterpTo` (`SceneComponent.K2_GetComponentLocation` _camera) (`SplineComponent.FindLocationClosestToWorldLocation` (`self.Spline`) (`self.K2_GetActorLocation` (`self.Character`)) "World") (`self.Delta Seconds`)) (`KismetMathLibrary.RInterpTo` (`SceneComponent.K2_GetComponentRotation` _camera) (`KismetMathLibrary.FindLookAtRotation` (`SceneComponent.K2_GetComponentLocation` (`self.Camera`)) (`self.K2_GetActorLocation`)) (`self.Delta Seconds`)) false false))))

(fn `UserConstructionScript`)