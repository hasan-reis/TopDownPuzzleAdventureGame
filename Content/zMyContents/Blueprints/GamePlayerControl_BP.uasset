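; Player control Blueprint for click-to-move and tap-based selection of Player_BP characters.
; While left mouse is held, a Tick-driven gate traces under the cursor and calls SimpleMoveToLocation beyond a minimum distance.
; Short first-finger taps on characters drive target icons and possession; only the no-selection branch blends to a camera volume, but it never assigns the tapped character.
; An equivalent touch-movement gate is left unconnected.
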(event `Key|LeftMouseButton`
  (params (Key :type "Key Structure"))
  (:`Pressed`
    (goto _label :!via `Open`))
  (:`Released`
    (goto _label :!via `Close`)))

(event `self.ReceiveTick`
  (params (DeltaSeconds :type "Float (single-precision)"))
  (`|ExecutionSequence`
    (:`then_0`
      (`/Engine/EditorBlueprintResources/StandardMacros.Gate` true :!label _label
        (:`Exit`
          (`self.MoveToHitResult` (`PlayerController.GetHitResultUnderCursorForObjects` (`GameplayStatics.GetPlayerController` 0) (`|MakeArray` "ObjectTypeQuery1" "ObjectTypeQuery2" :!type "EObjectTypeQuery Enum") true)))))))

(event `self.ReceiveBeginPlay`
  (set `PlayerController.bShowMouseCursor` true (`GameplayStatics.GetPlayerController` 0)))

(event `InputTouch`
  (params (Location :type "Vector Structure") (FingerIndex :type "ETouchIndex Enum"))
  ;[1 1 1] Parmakla bastigin yere hareket etmesi
  ;;[1 1 1 1 12] Pressed->Open Released->Close
)

(event `InputTouch`
  (params (Location :type "Vector Structure") (FingerIndex :type "ETouchIndex Enum"))
  (bind _returnvalue (`GameplayStatics.GetPlayerController` 0))
  (bind _returnvalue_2 (`|EnumEquality` FingerIndex "Touch1"))
  (bind _hitactor (`self.HitActor`))
  (bind _selectedcharacter (`self.SelectedCharacter`))
  (bind (_locationx _locationy) (`PlayerController.GetInputTouchState` (`GameplayStatics.GetPlayerController` 0) "Touch1"))
  (bind _returnvalue_3 (`KismetMathLibrary.MakeVector2D` _locationx _locationy))
  (:`Pressed`
    (if _returnvalue_2
      (bind _output_get (set `self.InitTouchLocation` _returnvalue_3))
      (set `self.HitActor` (`.HitActor` (`GameplayStatics.BreakHitResult` (`PlayerController.GetHitResultUnderFingerByChannel` (`GameplayStatics.GetPlayerController` 0) "Touch1" "TraceTypeQuery1" true))))))
  (:`Released`
    (if _returnvalue_2
      (bind _output_get_2 (set `self.FinalTouchLocation` _returnvalue_3))
      (if (< (`KismetMathLibrary.VSize2D` (- _output_get _output_get_2)) (`self.MinDragThresold`))
        (`/Engine/EditorBlueprintResources/StandardMacros.IsValid` _hitactor
          (:`Is Valid`
            (bind _asplayer_bp (cast `/Game/zMyContents/Blueprints/Player_BP` _hitactor))
            (set `self.HitCharacter` _asplayer_bp)
            (`/Engine/EditorBlueprintResources/StandardMacros.IsValid` _selectedcharacter
              (:`Is Valid`
                (`/Game/zMyContents/Blueprints/Player_BP.DisableTargetIcon` (`self.SelectedCharacter`))
                (`Controller.UnPossess` _returnvalue)
                (bind _output_get_3 (set `self.SelectedCharacter` (`self.HitCharacter`)))
                (`/Game/zMyContents/Blueprints/Player_BP.EnableTargetIcon` _output_get_3)
                (`Controller.Possess` _returnvalue _output_get_3))
              (:`Is Not Valid`
                (bind _output_get_4 (set `self.SelectedCharacter` _selectedcharacter))
                (`/Game/zMyContents/Blueprints/Player_BP.EnableTargetIcon` _output_get_4)
                (`Controller.Possess` _returnvalue _output_get_4)
                (`PlayerController.SetViewTargetWithBlend` _returnvalue (`/Game/zMyContents/Blueprints/Player_BP.CurrentCameraVolume` _output_get_4) 2.0 "VTBlend_Linear" 5.0 false)))))))))

(fn `MoveToHitResult`
  (params (`Hit Resut` :type "HitResult Structure"))
  (bind (_bblockinghit _binitialoverlap _time _distance _location) (`GameplayStatics.BreakHitResult` `Hit Resut`))
  (bind _returnvalue (`KismetMathLibrary.VSize` (- (`self.K2_GetActorLocation` (`GameplayStatics.GetPlayerPawn` 0)) _location)))
  (`KismetSystemLibrary.PrintString` (`KismetStringLibrary.Conv_DoubleToString` _returnvalue))
  (if (<= (`self.MinClickDistance`) _returnvalue)
    (`AIBlueprintHelperLibrary.SimpleMoveToLocation` null _location)))

(fn `UserConstructionScript`)